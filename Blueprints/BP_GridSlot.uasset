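; Clickable tile of a combat grid that stores its position and reports cursor hover to the owning Grid.
; Left click starts combat through Grid setup if not already running; other buttons spawn an entity.
; Helpers match units by position for lookup, AI movement and damage, though damage compares the requester to itself, so never applies.
; The click logic for selecting units and dispatching Move or Attack is disconnected.
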(event `Disable/EnableAction`
  (params (`Enable?` :type Boolean))
  ;[1 1 1] Enable clickable
  (set `self.InRangeForAction` `Enable?`))

(event `ChangeMaterial`
  (params (Material :type "MaterialInterface Object Reference"))
  ;[1 1 1] Change material to indicate cilckable
  (`PrimitiveComponent.SetMaterial` (`self.Cube`) 0 Material)
  (`KismetSystemLibrary.Delay` 2.0)
  (`PrimitiveComponent.SetMaterial` (`self.Cube`) 0 "/Game/Material/MI_GridTransparentGreen.MI_GridTransparentGreen"))

(event `self.ReceiveActorBeginCursorOver`
  ;[1 1 1] Indicate which slot that is being hovered
  (`/Game/Blueprints/BP_Grid.MoveSelectedSlot` (`self.Grid`) (`self.Position`)))

(event `self.ReceiveActorOnClicked`
  (params (ButtonPressed :type "Key Structure"))
  (bind _controller (`self.Controller`))
  (bind _controller_2 (`self.Controller`))
  (if (== ButtonPressed "LeftMouseButton")
    (`/Engine/EditorBlueprintResources/StandardMacros.IsValid` (`self.Controller`)
      (:`Is Valid`
        (if (not (`/Game/Blueprints/PC_PlayerController.InCombat` (`self.Controller`)))
          (`/Game/Blueprints/BP_Grid.Setup` (`self.Grid`) (`/Game/Blueprints/PC_PlayerController.TurnManager` _controller))
          (set `/Game/Blueprints/PC_PlayerController.InCombat` true _controller)))
      (:`Is Not Valid`
        (bind _aspc_player_controller (cast `/Game/Blueprints/PC_PlayerController` (`GameplayStatics.GetPlayerController` 0)))
        (bind _output_get (set `self.Controller` _aspc_player_controller))
        (if (not (`/Game/Blueprints/PC_PlayerController.InCombat` _output_get))
          (`/Game/Blueprints/BP_Grid.Setup` (`self.Grid`) (`/Game/Blueprints/PC_PlayerController.TurnManager` _controller_2))
          (set `/Game/Blueprints/PC_PlayerController.InCombat` true _controller_2))))
    (else
      ;[1 1 1] Spawn units
      (`/Game/Blueprints/BP_Grid.Add Entity` (`self.Grid`) false))))

(fn `CheckUnitOnGrid`
  (returns (FoundActor :type "Actor Object Reference"))
  (for _array_element (`/Game/Blueprints/BP_Grid.UnitsOnGrid` (`self.Grid`))
    (if (`KismetStringLibrary.EqualEqual_StrStr` (`/Game/Blueprints/BP_Entity.Position` _array_element) (`self.Position`))
      (return _array_element)))
  (return null))

(fn `DamageUnits`
  (params (RequestingUnit :type "/Game/Blueprints/BP_Entity Object Reference"))
  (for _array_element (`/Game/Blueprints/BP_Grid.UnitsOnGrid` (`self.Grid`))
    (if (`KismetStringLibrary.EqualEqual_StrStr` (`/Game/Blueprints/BP_Entity.Position` _array_element) (`self.Position`))
      (if (!= RequestingUnit (`local.RequestingUnit`))
        (`GameplayStatics.ApplyDamage` RequestingUnit (`KismetMathLibrary.Conv_IntToDouble` (`/Game/Blueprints/BP_Entity.attack` RequestingUnit)))
        (return)))))

(fn `MoveUnit`
  (params (RequestingUnit :type "/Game/Blueprints/BP_Entity Object Reference"))
  (bind _returnvalue (`SceneComponent.K2_GetComponentLocation` (`self.TargetPathfinding`)))
  (for _array_element (`/Game/Blueprints/BP_Grid.UnitsOnGrid` (`self.Grid`))
    (if (`KismetStringLibrary.EqualEqual_StrStr` (`/Game/Blueprints/BP_Entity.Position` _array_element) (`self.Position`))
      (return)))
  (bind _outhit (`KismetSystemLibrary.LineTraceSingle` _returnvalue (- _returnvalue (0.0 0.0 200.0)) "TraceTypeQuery1"))
  (`AIBlueprintHelperLibrary.SimpleMoveToLocation` (`/Game/Blueprints/BP_Entity.AIController` (`local.RequestingUnit`)) (`.Location` (`GameplayStatics.BreakHitResult` _outhit)))
  (set `/Game/Blueprints/BP_Entity.Position` (`self.Position`) (`local.RequestingUnit`))
  (`/Game/Blueprints/PC_PlayerController.ClearSelectUnit` (`self.Controller`))
  (`/Game/Blueprints/BP_Grid.ResetGridSlots` (`self.Grid`))
  (`self.ChangeMaterial` "/Game/Material/MI_GridTransparentGreen.MI_GridTransparentGreen"))

(fn `Setup`
  (params (Grid :type "/Game/Blueprints/BP_Grid Object Reference") (Position :type String) (Controller :type "/Game/Blueprints/PC_PlayerController Object Reference") (TurnManager :type "/Game/Blueprints/BP_TurnSystem Object Reference"))
  (set `self.Grid` Grid)
  (set `self.Position` Position)
  (set `self.Controller` Controller)
  (set `self.TurnManager` TurnManager))

(fn `UserConstructionScript`)