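; BP_Grid is a tile grid actor for placing, selecting and moving units in what appears to be a tactics game.
; Its construction script builds Size-based mesh tiles and sizes the IsiGrid occupancy array.
; Cursor traces move the selection marker or spawn a BP_Entity on right-click, while F selects the marked entity and updates the action bar.
; Green tile material marks valid move targets for units with an action, without updating IsiGrid.
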(event `self.ReceiveBeginPlay`
  (`PaperSpriteComponent.SetSpriteColor` :`self` (`self.SelectedSlot`))
  (bind _returnvalue (`|CreateWidget` "/Game/WB_ActionBar.WB_ActionBar_C"))
  (bind _output_get (set `self.ActionBar` _returnvalue))
  (`UserWidget.AddToViewport` _output_get 0))

(event `Key|LeftMouseButton`
  (params (Key :type "Key Structure"))
  (bind _selectedunit (`self.SelectedUnit`))
  (bind (_bblockinghit _binitialoverlap _time _distance _location _impactpoint _normal _impactnormal _physmat _hitactor _hitcomponent) (`GameplayStatics.BreakHitResult` (`PlayerController.GetHitResultUnderCursorByChannel` (`GameplayStatics.GetPlayerController` 0) "TraceTypeQuery3" true)))
  (bind _returnvalue (`SceneComponent.GetRelativeTransform` _hitcomponent))
  (bind _returnvalue_2 (`KismetMathLibrary.FTrunc` (/ (.x (.location _returnvalue)) 120.0)))
  (bind _returnvalue_3 (`KismetMathLibrary.FTrunc` (/ (.y (.location _returnvalue)) 120.0)))
  (:`Pressed`
    (`PaperSpriteComponent.SetSpriteColor` (`self.SelectedSlot`) (struct :`R` 1.0 :`G` 1.0 :`B` 1.0 :`A` 1.0))
    (cast `/Game/BP_Grid` _hitactor)
    (`SceneComponent.K2_SetRelativeLocation` (`self.SelectedSlot`) (`KismetMathLibrary.MakeVector` (.x (.location _returnvalue)) (.y (.location _returnvalue)) (`.Z` (`KismetMathLibrary.BreakVector3f` (`SceneComponent.RelativeLocation` (`self.SelectedSlot`))))) false true)
    (`KismetSystemLibrary.PrintString` (`KismetStringLibrary.Conv_DoubleToString` (/ (.x (.location _returnvalue)) 120.0)))
    (`KismetSystemLibrary.PrintString` (`KismetStringLibrary.Conv_DoubleToString` (/ (.y (.location _returnvalue)) 120.0)))
    (if (== (`PrimitiveComponent.GetMaterial` _hitcomponent 0) "/AnimationSharing/AnimSharingGreen.AnimSharingGreen")
      (`/Engine/EditorBlueprintResources/StandardMacros.IsValid` _selectedunit
        (:`Is Valid`
          (if (not (`KismetStringLibrary.IsEmpty` (`.Name_10_5A17C7AB464443F7A45668BBD43A2064` (break `/Game/S_Action` (`/Game/BP_Entity.Selected Action` _selectedunit)))))
            (`self.K2_SetActorLocation` (`self.SelectedUnit`) (+ (`SceneComponent.K2_GetComponentLocation` (`|GetArrayItem` (`self.GridSlots`) (+ _returnvalue_2 (* _returnvalue_3 (`|GetArrayItem` (`self.Size`)))))) (0.0 0.0 50.0)) false false)
            (set `/Game/BP_Entity.Position` (`|MakeArray` _returnvalue_2 _returnvalue_3) (`self.SelectedUnit`))
            (set `/Game/BP_Entity.Selected Action` (struct) (`self.SelectedUnit`))
            (for _array_element (`self.GridSlots`)
              (`PrimitiveComponent.SetMaterial` _array_element 0 "/Engine/EngineMaterials/DefaultMaterial.DefaultMaterial"))))))))

(event `Key|RightMouseButton`
  (params (Key :type "Key Structure"))
  (bind (_bblockinghit _binitialoverlap _time _distance _location _impactpoint _normal _impactnormal _physmat _hitactor _hitcomponent) (`GameplayStatics.BreakHitResult` (`PlayerController.GetHitResultUnderCursorByChannel` (`GameplayStatics.GetPlayerController` 0) "TraceTypeQuery3" true)))
  (bind _returnvalue (`SceneComponent.GetRelativeTransform` _hitcomponent))
  (:`Pressed`
    (cast `/Game/BP_Grid` _hitactor)
    (`self.Add Entity` (`KismetMathLibrary.FTrunc` (/ (.x (.location _returnvalue)) 120.0)) (`KismetMathLibrary.FTrunc` (/ (.y (.location _returnvalue)) 120.0)))))

(event `Add Entity`
  (params (PosX :type Integer) (PosY :type Integer))
  (bind _returnvalue (+ PosX (* PosY (`|GetArrayItem` (`self.Size`)))))
  (bind _returnvalue_2 (`|SpawnActorFromClass` "/Game/BP_Entity.BP_Entity_C" (`KismetMathLibrary.MakeTransform` (+ (`SceneComponent.K2_GetComponentLocation` (`|GetArrayItem` (`self.GridSlots`) _returnvalue)) (0.0 0.0 50.0))) "Undefined" "MultiplyWithRoot" null (`|MakeArray` PosX PosY) self null))
  (`KismetArrayLibrary.Array_Set` (`self.isi Grid`) _returnvalue _returnvalue_2))

(event `Key|F`
  (params (Key :type "Key Structure"))
  (:`Pressed`
    (bind (_outactors _returnvalue) (`KismetSystemLibrary.BoxOverlapActors` (`SceneComponent.K2_GetComponentLocation` (`self.SelectedSlot`)) (30.0 30.0 30.0) (`|MakeArray` "ObjectTypeQuery2" :!type "EObjectTypeQuery Enum") "/Game/BP_Entity.BP_Entity_C"))
    (if _returnvalue
      (for _array_element _outactors
        (bind _asbp_entity (cast `/Game/BP_Entity` _array_element))
        (bind _output_get (set `self.SelectedUnit` _asbp_entity))
        (`/Game/BP_Entity.ChangeMaterial` _output_get "/AnimationSharing/AnimSharingGreen.AnimSharingGreen")
        (`/Game/WB_ActionBar.UpdateSelectedUnit` (`self.ActionBar`) (`self.SelectedUnit`)))
      (else
        (`/Engine/EditorBlueprintResources/StandardMacros.IsValid` (`self.SelectedUnit`)
          (:`Is Valid`
            (`/Game/BP_Entity.ChangeMaterial` (`self.SelectedUnit`) "/Engine/MapTemplates/Materials/BasicAsset01.BasicAsset01")
            (set `self.SelectedUnit` null)))))))

(fn `UserConstructionScript`
  (bind _isi_grid (`self.isi Grid`))
  (for _index (range (`|GetArrayItem` (`self.Size`) 1))
    (for _index_2 (range (`|GetArrayItem` (`self.Size`)))
      (bind _returnvalue (`AddComponent|NODE_AddStaticMeshComponent-2` :`RelativeTransform` (`KismetMathLibrary.MakeTransform` (`KismetMathLibrary.MakeVector` (`KismetMathLibrary.Conv_IntToDouble` (* _index_2 120)) (`KismetMathLibrary.Conv_IntToDouble` (* _index 120)) -45.0))))
      (`KismetArrayLibrary.Array_AddUnique` (`self.GridSlots`) _returnvalue)))
  (`KismetArrayLibrary.Array_Resize` _isi_grid (* (`|GetArrayItem` (`self.Size`)) (`|GetArrayItem` (`self.Size`) 1)))
  (`KismetSystemLibrary.PrintString` (`KismetSystemLibrary.GetDisplayName` (`|GetArrayItem` _isi_grid))))