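; AC_Basic is an AI controller for pawns that act in turns.
; On possession it runs the BT_Base behavior tree and sets the blackboard's Turn key to false.
; Its ChangeTurn event writes CanMove into that key, exposing turn state to the tree, and prints the controlled pawn's name.
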(event `self.ReceivePossess`
  (params (PossessedPawn :type "Pawn Object Reference"))
  (`self.RunBehaviorTree` "/Game/Blueprints/AI/BehaviorTree/BT_Base.BT_Base")
  (`BlackboardComponent.SetValueAsBool` (`AIBlueprintHelperLibrary.GetBlackboard` null) "Turn" false))

(event `ChangeTurn`
  (params (`CanMove?` :type Boolean))
  (`KismetSystemLibrary.PrintString` (`KismetSystemLibrary.GetDisplayName` (`self.K2_GetPawn`)))
  (`BlackboardComponent.SetValueAsBool` (`AIBlueprintHelperLibrary.GetBlackboard` null) "Turn" `CanMove?`))

(fn `UserConstructionScript`)