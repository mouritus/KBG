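; Grid unit for a turn-based game that takes damage and passes turn changes to its AC_Basic AI controller.
; On BeginPlay, a non-copy grabs the Grid's TurnManager and spawns a flagged duplicate of itself far below.
; Damage lowers health, shrinking the cube when low, and destruction removes the unit from the Grid.
; Tick snaps sprite rotation by yaw; GetGridInfo returns slots and other units' positions; Monte Carlo search debugging is unwired.
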(event `self.ReceiveBeginPlay`
  (if (not (`self.IsCopy?`))
    (set `self.Turn Manager` (`/Game/Blueprints/BP_Grid.TurnManager` (`self.Grid`)))
    (bind _returnvalue (`|SpawnActorFromClass` (`GameplayStatics.GetObjectClass` self) (`KismetMathLibrary.MakeTransform` (- (`self.K2_GetActorLocation` self) (0.0 0.0 1000.0))) "Undefined" "MultiplyWithRoot" null null "0102" true null))
    (set `self.Copy` _returnvalue)))

(event `ChangeMaterial`
  (params (`New Material` :type "MaterialInterface Object Reference"))
  (`PrimitiveComponent.SetMaterial` (`self.Cube`) 0 `New Material`))

(event `self.ReceiveAnyDamage`
  (params (Damage :type "Float (single-precision)") (DamageType :type "DamageType Object Reference") (InstigatedBy :type "Controller Object Reference") (DamageCauser :type "Actor Object Reference"))
  (`KismetSystemLibrary.PrintString` (`KismetStringLibrary.Concat_StrStr` (`KismetSystemLibrary.GetDisplayName` self) ": got hit"))
  (`NiagaraFunctionLibrary.SpawnSystemAtLocation` null (`self.K2_GetActorLocation`))
  (bind _output_get (set `self.health` (`KismetMathLibrary.Clamp` (`KismetMathLibrary.FTrunc` (- (`self.health`) Damage)) 0 (`self.health`))))
  (if (<= _output_get 0)
    (`self.K2_DestroyActor`)
    (elif (<= _output_get 5)
      (`SceneComponent.SetRelativeScale3D` (`self.Cube`) (0.5 0.5 0.5)))))

(event `ChangeTurn`
  (params (`CanMove?` :type Boolean))
  (`/Engine/EditorBlueprintResources/StandardMacros.IsValid` (`self.AIController`)
    (:`Is Valid`
      _)
    (:`Is Not Valid`
      (bind _asac_basic (cast `/Game/Blueprints/AI/Controller/AC_Basic` (`AIBlueprintHelperLibrary.GetAIController` self)))
      (set `self.AIController` _asac_basic)))
  (`/Game/Blueprints/AI/Controller/AC_Basic.ChangeTurn` (`self.AIController`) `CanMove?`))

(event `self.ReceiveDestroyed`
  (`/Game/Blueprints/BP_Grid.RemoveUnit` (`self.Grid`) self))

(event `Use Monte Carlo`)

(event `self.ReceiveTick`
  (params (DeltaSeconds :type "Float (single-precision)"))
  (bind (_returnvalue_roll _returnvalue_pitch _returnvalue_yaw) (`KismetMathLibrary.BreakRotator` (`self.K2_GetActorRotation`)))
  (if (or (>= _returnvalue_yaw -0.1) (<= _returnvalue_yaw -179.9))
    (`SceneComponent.K2_SetWorldRotation` (`self.Sprite`) (struct :`Yaw` 90.0) false false)
    (else
      (`SceneComponent.K2_SetWorldRotation` (`self.Sprite`) (struct :`Yaw` 270.0) false false))))

(fn `GetGridInfo`
  (returns (GridPositions :type "Array of String") (UnitPositions :type "Array of String"))
  (locals (FoundUnitPositions :type "Array of String"))
  (bind _grid (`self.Grid`))
  (bind _unitsongrid (`/Game/Blueprints/BP_Grid.UnitsOnGrid` _grid))
  (`/Engine/EditorBlueprintResources/StandardMacros.IsValid` _grid
    (:`Is Valid`
      (`KismetArrayLibrary.Array_Clear` (`local.FoundUnitPositions`))
      (for (_array_element _array_index) _unitsongrid
        (if (!= _array_index (`KismetArrayLibrary.Array_Find` _unitsongrid self))
          (`KismetArrayLibrary.Array_Add` (`local.FoundUnitPositions`) (`/Game/Blueprints/BP_Entity.Position` _array_element))))
      (bind _keys (`BlueprintMapLibrary.Map_Keys` (`/Game/Blueprints/BP_Grid.GridSlots` _grid)))
      (return _keys (`local.FoundUnitPositions`)))))

(fn `UserConstructionScript`)