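; Player controller for a grid-based game that tracks the selected unit and action.
; On BeginPlay it shows the cursor and adds the WB_ActionBar widget to the viewport.
; Selection events swap the unit's material as a highlight and update the action bar.
; Choosing an action resets the grid slots, then has the externally supplied grid reference check that action's range from the unit's position.
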(event `self.ReceiveBeginPlay`
  (set `self.bShowMouseCursor` true)
  (bind _returnvalue (`|CreateWidget` "/Game/Widgets/WB_ActionBar.WB_ActionBar_C" null self))
  (bind _output_get (set `self.ActionBar` _returnvalue))
  (`UserWidget.AddToViewport` _output_get 0))

(event `UpdateGridRef`
  (params (Ref_Grid :type "/Game/Blueprints/BP_Grid Object Reference"))
  (set `self.Ref_Grid` Ref_Grid))

(event `SelectUnit`
  (params (Unit :type "/Game/Blueprints/BP_Entity Object Reference"))
  (bind _output_get (set `self.SelectedUnit` Unit))
  (`/Game/Blueprints/BP_Entity.ChangeMaterial` _output_get "/AnimationSharing/AnimSharingGreen.AnimSharingGreen")
  (`/Game/Widgets/WB_ActionBar.UpdateSelectedUnit` (`self.ActionBar`) (`self.SelectedUnit`)))

(event `ClearSelectUnit`
  (`/Engine/EditorBlueprintResources/StandardMacros.IsValid` (`self.SelectedUnit`)
    (:`Is Valid`
      (`/Game/Blueprints/BP_Entity.ChangeMaterial` (`self.SelectedUnit`) "/Engine/MapTemplates/Materials/BasicAsset01.BasicAsset01"))
    (:`Is Not Valid`
      _))
  (set `self.SelectedUnit` null)
  (set `self.SelectedAction` (struct))
  (`/Game/Widgets/WB_ActionBar.UpdateSelectedUnit` (`self.ActionBar`) null))

(event `SelectAction`
  (params (SelectedAction :type "/Game/Structures/S_Action Structure"))
  (`/Game/Blueprints/BP_Grid.ResetGridSlots` (`self.Ref_Grid`))
  (bind _output_get (set `self.SelectedAction` SelectedAction))
  (`/Game/Blueprints/BP_Grid.CheckActionRange` (`self.Ref_Grid`) _output_get (`/Game/Blueprints/BP_Entity.Position` (`self.SelectedUnit`))))

(fn `UserConstructionScript`)