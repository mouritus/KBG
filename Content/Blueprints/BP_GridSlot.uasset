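; BP_GridSlot is a clickable tile in a grid-based unit game that reports hover to its Grid.
; Left-click runs the selected unit's Move or Attack when the slot is in range, otherwise it selects any BP_Entity standing there; other clicks spawn entities through the Grid.
; Box overlaps detect occupants, so moves teleport only onto empty slots and attacks damage nearby entities except the attacker.
; Resolved actions clear selection and reset the grid.
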(event `Disable/EnableAction`
  (params (`Enable?` :type Boolean))
  ;[1 1 1] Enable clickable
  (set `self.InRangeForAction` `Enable?`))

(event `ChangeMaterial`
  (params (Material :type "MaterialInterface Object Reference"))
  ;[1 1 1] Change material to indicate cilckable
  (`PrimitiveComponent.SetMaterial` (`self.Cube`) 0 Material))

(event `self.ReceiveActorBeginCursorOver`
  ;[1 1 1] Indicate which slot that is being hovered
  (`/Game/Blueprints/BP_Grid.MoveSelectedSlot` (`self.Grid`) (`self.Position`)))

(event `self.ReceiveActorOnClicked`
  (params (ButtonPressed :type "Key Structure"))
  (bind _grid (`self.Grid`))
  (bind _selectedunit (`/Game/Blueprints/PC_PlayerController.SelectedUnit` (`self.Controller`)))
  (if (== ButtonPressed "LeftMouseButton")
    ;[1 1 1] Click events when the player is controlling a unit
    (if (`self.InRangeForAction`)
      (switch `string` (`.Name_10_5A17C7AB464443F7A45668BBD43A2064` (break `/Game/Structures/S_Action` (`/Game/Blueprints/PC_PlayerController.SelectedAction` (`self.Controller`))))
        (:`Move`
          (`self.MoveUnit` _selectedunit))
        (:`Attack`
          (`self.DamageUnits` _selectedunit)))
      (else
        ;[1 1 1] Control a unit
        (`/Game/Blueprints/PC_PlayerController.ClearSelectUnit` (`self.Controller`))
        (`/Game/Blueprints/BP_Grid.ResetGridSlots` (`self.Grid`))
        (bind (_outactors _returnvalue) (`KismetSystemLibrary.BoxOverlapActors` (`SceneComponent.K2_GetComponentLocation` (`self.Cube`)) (30.0 30.0 30.0) (`|MakeArray` "ObjectTypeQuery2" :!type "EObjectTypeQuery Enum") "/Game/Blueprints/BP_Entity.BP_Entity_C"))
        (if _returnvalue
          (for _array_element _outactors
            (bind _asbp_entity (cast `/Game/Blueprints/BP_Entity` _array_element))
            (`/Game/Blueprints/PC_PlayerController.SelectUnit` (`self.Controller`) _asbp_entity)))))
    (else
      ;[1 1 1] Spawn units
      (if (== ButtonPressed "RightMouseButton")
        (`/Game/Blueprints/BP_Grid.Add Entity` _grid false)
        (else
          (`/Game/Blueprints/BP_Grid.Add Entity` _grid true))))))

(fn `CheckUnitOnGrid`
  (returns (FoundActor :type "Array of Actor Object Reference"))
  (bind (_returnvalue_x _returnvalue_y _returnvalue_z) (`KismetMathLibrary.BreakVector` (`self.K2_GetActorLocation` self)))
  (bind _outactors (`KismetSystemLibrary.BoxOverlapActors` (`KismetMathLibrary.MakeVector` _returnvalue_x _returnvalue_y (+ _returnvalue_z 50.0)) (75.0 75.0 75.0) (`|MakeArray` "ObjectTypeQuery2" "ObjectTypeQuery1" :!type "EObjectTypeQuery Enum") "/Game/Blueprints/BP_Entity.BP_Entity_C"))
  (return _outactors))

(fn `DamageUnits`
  (params (RequestingUnit :type "/Game/Blueprints/BP_Entity Object Reference"))
  (bind (_returnvalue_x _returnvalue_y _returnvalue_z) (`KismetMathLibrary.BreakVector` (`self.K2_GetActorLocation` self)))
  (bind _outactors (`KismetSystemLibrary.BoxOverlapActors` (`KismetMathLibrary.MakeVector` _returnvalue_x _returnvalue_y (+ _returnvalue_z 50.0)) (75.0 75.0 75.0) (`|MakeArray` "ObjectTypeQuery2" :!type "EObjectTypeQuery Enum") "/Game/Blueprints/BP_Entity.BP_Entity_C"))
  (for _array_element _outactors
    (if (!= _array_element (`local.RequestingUnit`))
      (`GameplayStatics.ApplyDamage` _array_element 5.0)))
  (`/Game/Blueprints/PC_PlayerController.ClearSelectUnit` (`self.Controller`))
  (`/Game/Blueprints/BP_Grid.ResetGridSlots` (`self.Grid`)))

(fn `MoveUnit`
  (params (RequestingUnit :type "/Game/Blueprints/BP_Entity Object Reference"))
  (bind (_returnvalue_x _returnvalue_y _returnvalue_z) (`KismetMathLibrary.BreakVector` (`self.K2_GetActorLocation` self)))
  (bind (_returnvalue_x_2 _returnvalue_y_2 _returnvalue_z_2) (`KismetMathLibrary.BreakVector` (`self.K2_GetActorLocation` self)))
  (bind (_outactors _returnvalue) (`KismetSystemLibrary.BoxOverlapActors` (`KismetMathLibrary.MakeVector` _returnvalue_x_2 _returnvalue_y_2 (+ _returnvalue_z_2 50.0)) (75.0 75.0 75.0) (`|MakeArray` "ObjectTypeQuery2" :!type "EObjectTypeQuery Enum") "/Game/Blueprints/BP_Entity.BP_Entity_C"))
  (if (not _returnvalue)
    (`self.K2_SetActorLocation` (`local.RequestingUnit`) (`KismetMathLibrary.MakeVector` _returnvalue_x _returnvalue_y (+ _returnvalue_z 50.0)) false true)
    (set `/Game/Blueprints/BP_Entity.Position` (`self.Position`) (`local.RequestingUnit`))
    (`/Game/Blueprints/PC_PlayerController.ClearSelectUnit` (`self.Controller`))
    (`/Game/Blueprints/BP_Grid.ResetGridSlots` (`self.Grid`))))

(fn `Setup`
  (params (Grid :type "/Game/Blueprints/BP_Grid Object Reference") (Position :type String) (Controller :type "/Game/Blueprints/PC_PlayerController Object Reference") (TurnManager :type "/Game/Blueprints/BP_TurnSystem Object Reference"))
  (set `self.Grid` Grid)
  (set `self.Position` Position)
  (set `self.Controller` Controller)
  (set `self.TurnManager` TurnManager))

(fn `UserConstructionScript`)