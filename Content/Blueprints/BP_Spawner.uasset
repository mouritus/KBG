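; Spawner actor that populates a bounds volume with instances of a chosen class, up to a maximum count.
; On BeginPlay it spawns a starting batch, then a looping timer calls SpawnObject until the cap clears it; StartSpawning? restarts the timer.
; SpawnObject traces downward from random box points to place objects just above static ground, falling back to a random point in the box.
; Each spawned actor is tracked and receives a reference to the spawner.
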(event `self.ReceiveBeginPlay`
  (for _ (range (+ (`self.StartingObjects`) 1))
    (if (< (`KismetArrayLibrary.Array_Length` (`self.Objects`)) (`self.MaxObjects`))
      (`self.SpawnObject`)))
  (bind _returnvalue (`KismetSystemLibrary.K2_SetTimer` null "SpawnObject" (`self.RespawnTime`) true :!label _label))
  (set `self.Spawner` _returnvalue))

(event `StartSpawning?`
  (goto _label))

(fn `SpawnObject`
  (bind (_origin _boxextent) (`KismetSystemLibrary.GetComponentBounds` (`self.Bounds`)))
  (bind (_origin_2 _boxextent_2) (`KismetSystemLibrary.GetComponentBounds` (`self.Bounds`)))
  (bind _returnvalue (`KismetMathLibrary.RandomPointInBoundingBox` _origin_2 _boxextent_2))
  (if (< (`KismetArrayLibrary.Array_Length` (`self.Objects`)) (`self.MaxObjects`))
    ;[1 0.3099 0.2001] Get a random point in a bounding box and raycast to the floor so we can spawn stuff on the floor
    (bind (_outhit _returnvalue_2) (`KismetSystemLibrary.LineTraceSingleForObjects` _returnvalue (+ _returnvalue (* (* (`self.GetActorUpVector`) -100.0) (`.Z` (`KismetMathLibrary.BreakVector3f` _boxextent_2)))) (`|MakeArray` "ObjectTypeQuery1" :!type "EObjectTypeQuery Enum") true))
    (if _returnvalue_2
      (bind (_x _y _z) (`KismetMathLibrary.BreakVector3f` (`.ImpactPoint` (`GameplayStatics.BreakHitResult` _outhit))))
      (bind _returnvalue_3 (`|SpawnActorFromClass` (`self.SpawnedObject`) (`KismetMathLibrary.MakeTransform` (`KismetMathLibrary.MakeVector` _x _y (+ _z 10.0))) "Undefined" "MultiplyWithRoot" null null))
      (`KismetArrayLibrary.Array_Add` (`self.Objects`) _returnvalue_3)
      (message `/Game/Blueprints/BPI_Spawner.SetSpawner` _returnvalue_3 self)
      (else
        (bind _returnvalue_4 (`|SpawnActorFromClass` (`self.SpawnedObject`) (`KismetMathLibrary.MakeTransform` (`KismetMathLibrary.RandomPointInBoundingBox` _origin _boxextent)) "Undefined" "MultiplyWithRoot" null null))
        (`KismetArrayLibrary.Array_Add` (`self.Objects`) _returnvalue_4)
        (message `/Game/Blueprints/BPI_Spawner.SetSpawner` _returnvalue_4 self)))
    (else
      (`KismetSystemLibrary.K2_ClearAndInvalidateTimerHandle` (`self.Spawner`)))))

(fn `UserConstructionScript`)