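; Turn manager that cycles the active turn through registered units and can request an MCTS-based AI decision.
; Units live in a map to a has-turn flag, and a looping one-second timer runs NextTurn to pass that flag on, wrapping around.
; RequestMCTS flattens unit IDs, teams, grid positions and attack ranges into primitive arrays for SimulateAI, then only prints the returned action.
; Its sorted turn queue and separate teams array are never properly fed into the simulation.
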(event `StartTurnBase`
  ;[1 1 1] Enable turn to be changed
  (bind _keys (`BlueprintMapLibrary.Map_Keys` (`self.Units`)))
  (if (`KismetArrayLibrary.Array_IsNotEmpty` _keys)
    (`/Game/Blueprints/BP_Entity.ChangeTurn` (`|GetArrayItem` _keys) true)
    (set `self.TurnEnabled` true)
    (bind _returnvalue (`KismetSystemLibrary.K2_SetTimer` null "NextTurn" 1.0 true))
    (set `self.TurnSystem` _returnvalue)))

(event `AddUnit`
  (params (Unit :type "/Game/Blueprints/BP_Entity Object Reference (by ref)"))
  ;[1 1 1] Add unit to the turn system
  (if (`BlueprintMapLibrary.Map_IsEmpty` (`self.Units`))
    (`BlueprintMapLibrary.Map_Add` (`self.Units`) Unit true)
    (else
      (`BlueprintMapLibrary.Map_Add` (`self.Units`) Unit))))

(event `RemoveUnit`
  (params (Key :type "/Game/Blueprints/BP_Entity Object Reference (by ref)"))
  (`BlueprintMapLibrary.Map_Remove` (`self.Units`) Key))

(fn `NextTurn`
  (bind _units (`self.Units`))
  ;[1 1 1] Find who's turn is it
  (bind _keys (`BlueprintMapLibrary.Map_Keys` (`self.Units`)))
  (for (_array_element _array_index) _keys
    (if (`BlueprintMapLibrary.Map_Find` (`self.Units`) _array_element)
      ;[1 1 1] Change Turn
      (`/Game/Blueprints/BP_Entity.ChangeTurn` _array_element false)
      (`BlueprintMapLibrary.Map_Add` (`self.Units`) _array_element)
      (if (== _array_index (- (`KismetArrayLibrary.Array_Length` _keys) 1))
        (bind _output (`|GetArrayItem` _keys))
        (`BlueprintMapLibrary.Map_Add` _units _output true)
        (`/Game/Blueprints/BP_Entity.ChangeTurn` _output true)
        (break)
        (else
          (bind _output_2 (`|GetArrayItem` _keys (+ _array_index 1)))
          (`BlueprintMapLibrary.Map_Add` _units _output_2 true)
          (`/Game/Blueprints/BP_Entity.ChangeTurn` _output_2 true)
          (break))))))

(fn `RequestMCTS`
  (params (RequestingUnit :type "/Game/Blueprints/BP_Entity Object Reference"))
  (locals (UnsortedUnit :type "Array of /Game/Blueprints/BP_Entity Object Reference") (NextUnitTurn :type "/Game/Blueprints/BP_Entity Object Reference") (NextUnitIndex :type Integer) (SortedUnits :type "Array of /Game/Blueprints/BP_Entity Object Reference") (InputNPC :type "Array of Integer") (InputNPCTeams :type "Array of Integer") (InputPosX :type "Array of Integer") (InputPosY :type "Array of Integer") (InputAttackRangeX :type "Array of Integer") (InputAttackRangeY :type "Array of Integer"))
  (bind _nextunitindex (`local.NextUnitIndex`))
  (`KismetArrayLibrary.Array_Clear` (`local.SortedUnits`))
  (set `local.NextUnitIndex` -1)
  (bind _keys (`BlueprintMapLibrary.Map_Keys` (`self.Units`)))
  (bind _output_get (set `local.UnsortedUnit` _keys))
  (for (_array_element _array_index) _output_get
    ;[1 0.2661 0.6892] Find whose turn is it
    (if (`BlueprintMapLibrary.Map_Find` (`self.Units`) _array_element)
      (bind _output_get_2 (set `local.NextUnitTurn` _array_element))
      (set `local.NextUnitIndex` _array_index)
      (`KismetArrayLibrary.Array_Add` (`local.SortedUnits`) _output_get_2)
      (else
        ;[1 1 1] Add the next units in the turn queue
        (if (and (> _array_index _nextunitindex) (> _nextunitindex 0))
          (`KismetArrayLibrary.Array_Add` (`local.SortedUnits`) _array_element)))))
  ;[0.4242 0.4081 1] Add units from the one before the selected unit
  (for _index (range (+ (`local.NextUnitIndex`) 1))
    (bind _output (`|GetArrayItem` (`local.UnsortedUnit`) _index))
    (if (< (`KismetArrayLibrary.Array_Find` (`local.SortedUnits`) _output) 0)
      (`KismetArrayLibrary.Array_Add` (`local.SortedUnits`) _output)))
  ;[1 1 1] Setup primitives for input
  (`KismetArrayLibrary.Array_Clear` (`local.InputNPC`))
  (`KismetArrayLibrary.Array_Clear` (`local.InputNPCTeams`))
  (`KismetArrayLibrary.Array_Clear` (`local.InputPosX`))
  (`KismetArrayLibrary.Array_Clear` (`local.InputPosY`))
  (`KismetArrayLibrary.Array_Clear` (`local.InputAttackRangeX`))
  (`KismetArrayLibrary.Array_Clear` (`local.InputAttackRangeY`))
  (for _array_element_2 (`local.UnsortedUnit`)
    (`KismetArrayLibrary.Array_Add` (`local.InputNPC`) (`/Game/Blueprints/BP_Entity.ID` _array_element_2))
    (if (`/Game/Blueprints/BP_Entity.Ally?` _array_element_2)
      (`KismetArrayLibrary.Array_Add` (`local.InputNPC`) 1)
      (else
        (`KismetArrayLibrary.Array_Add` (`local.InputNPC`) -1)))
    (bind _position (`/Game/Blueprints/BP_Entity.Position` _array_element_2))
    (`KismetArrayLibrary.Array_Add` (`local.InputPosX`) (`KismetStringLibrary.Conv_StringToInt` (`KismetStringLibrary.GetSubstring` _position 0 2)))
    (`KismetArrayLibrary.Array_Add` (`local.InputPosY`) (`KismetStringLibrary.Conv_StringToInt` (`KismetStringLibrary.GetSubstring` _position 2 2)))
    (bind (_name _targetsize) (break `/Game/Structures/S_Action` (`|GetArrayItem` (`/Game/Blueprints/BP_Entity.Actions` _array_element_2) 1)))
    (`KismetArrayLibrary.Array_Add` (`local.InputAttackRangeX`) (`|GetArrayItem` _targetsize))
    (`KismetArrayLibrary.Array_Add` (`local.InputAttackRangeY`) (`|GetArrayItem` _targetsize)))
  ;[0.1051 0.4063 1] Simulate MCTS
  (bind _actiontaken (`MCTS_Functions.SimulateAI` (`local.InputNPC`) (`local.InputNPCTeams`) (`local.InputPosX`) (`local.InputPosY`) (`local.InputAttackRangeX`) (`local.InputAttackRangeY`)))
  (`KismetSystemLibrary.PrintString` (`KismetStringLibrary.Concat_StrStr` "Action taken is: " (`KismetStringLibrary.Conv_IntToString` _actiontaken)) true true (struct :`R` 1.0 :`B` 0.055357 :`A` 1.0) 5.0))

(fn `SetUp`
  (params (Grid :type "/Game/Blueprints/BP_Grid Object Reference"))
  (set `self.Grid` Grid))

(fn `UserConstructionScript`)