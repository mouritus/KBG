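; BP_Entity is a grid-based actor with health that can preview the range of a selected action.
; CheckActionRange loops over slots around its Position, clamped to the grid bounds, coloring occupied ones red and free ones green.
; Occupancy comes from a box overlap at each slot's location, filtered to other BP_Entity actors.
; Damage lowers Health, turning the cube red when low and destroying the actor at zero.
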(event `ChangeMaterial`
  (params (`New Material` :type "MaterialInterface Object Reference"))
  (`PrimitiveComponent.SetMaterial` (`self.Cube`) 0 `New Material`))

(event `self.ReceiveAnyDamage`
  (params (Damage :type "Float (single-precision)") (DamageType :type "DamageType Object Reference") (InstigatedBy :type "Controller Object Reference") (DamageCauser :type "Actor Object Reference"))
  (bind _output_get (set `self.health` (`KismetMathLibrary.Clamp` (`KismetMathLibrary.FTrunc` (- (`self.health`) Damage)) 0 (`self.health`))))
  (if (<= _output_get 0)
    (`self.K2_DestroyActor`)
    (elif (<= _output_get 5)
      (`self.ChangeMaterial` "/AnimationSharing/AnimSharingRed.AnimSharingRed"))))

(fn `CheckActionRange`
  (params (SelectedAction :type "/Game/S_Action Structure"))
  (bind (_targetsize _range) (break `/Game/S_Action` SelectedAction))
  (bind _output (`|GetArrayItem` _range))
  (bind _output_2 (`|GetArrayItem` (`self.Position`)))
  (bind _output_3 (`|GetArrayItem` (`self.Position`) 1))
  (bind _output_4 (`|GetArrayItem` _range 1))
  (set `self.Selected Action` SelectedAction)
  (for _index (range (`KismetMathLibrary.Clamp` (- _output_3 _output_4) 0 (- (`|GetArrayItem` (`/Game/BP_Grid.Size` (`self.Grid`)) 1) 1)) (+ (`KismetMathLibrary.Clamp` (+ _output_3 _output_4) 0 (- (`|GetArrayItem` (`/Game/BP_Grid.Size` (`self.Grid`)) 1) 1)) 1))
    (for _index_2 (range (`KismetMathLibrary.Clamp` (- _output_2 _output) 0 (- (`|GetArrayItem` (`/Game/BP_Grid.Size` (`self.Grid`))) 1)) (+ (`KismetMathLibrary.Clamp` (+ _output_2 _output) 0 (- (`|GetArrayItem` (`/Game/BP_Grid.Size` (`self.Grid`))) 1)) 1))
      (bind _returnvalue (+ (* (`|GetArrayItem` (`/Game/BP_Grid.Size` (`self.Grid`))) _index) _index_2))
      (bind _output_5 (`|GetArrayItem` (`/Game/BP_Grid.GridSlots` (`self.Grid`)) _returnvalue))
      (`/Engine/EditorBlueprintResources/StandardMacros.IsValid` _output_5
        (:`Is Valid`
          (if (`self.CheckIfSlotIsOccupied` _returnvalue)
            (`PrimitiveComponent.SetMaterial` _output_5 0 "/AnimationSharing/AnimSharingRed.AnimSharingRed")
            (else
              (`PrimitiveComponent.SetMaterial` _output_5 0 "/AnimationSharing/AnimSharingGreen.AnimSharingGreen"))))))))

(fn `CheckIfSlotIsOccupied`
  (params (Position :type Integer))
  (returns (`FoundUnit?` :type Boolean))
  (bind (_outactors _returnvalue) (`KismetSystemLibrary.BoxOverlapActors` (`SceneComponent.K2_GetComponentLocation` (`|GetArrayItem` (`/Game/BP_Grid.GridSlots` (`self.Grid`)) Position)) (30.0 30.0 30.0) (`|MakeArray` "ObjectTypeQuery2" :!type "EObjectTypeQuery Enum") "BP_Entity_C"))
  (return _returnvalue))

(fn `UserConstructionScript`)